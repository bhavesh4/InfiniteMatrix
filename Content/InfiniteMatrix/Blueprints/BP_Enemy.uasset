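; BP_Enemy is a short-lived enemy actor that damages the player on contact and can be destroyed by projectiles.
; Overlapping a BP_Player calls its ProcessHit and destroys the enemy, while overlapping a BP_Projectile destroys both actors.
; It records its start time on BeginPlay and checks the elapsed time every Tick to destroy itself after a fixed five-second lifetime.
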(event `self.ReceiveActorBeginOverlap`
  (params (OtherActor :type "Actor Object Reference"))
  (bind _asbp_player (cast `/Game/InfiniteMatrix/Blueprints/BP_Player` OtherActor)
    (:`then`
      (`/Game/InfiniteMatrix/Blueprints/BP_Player.ProcessHit` _asbp_player)
      (`self.K2_DestroyActor`))
    (:`CastFailed`
      (bind _asbp_projectile (cast `/Game/InfiniteMatrix/Blueprints/BP_Projectile` OtherActor))
      (`self.K2_DestroyActor` _asbp_projectile)
      (`self.K2_DestroyActor`))))

(event `self.ReceiveBeginPlay`
  (set `self.startTime` (`self.GetGameTimeSinceCreation`)))

(event `self.ReceiveTick`
  (params (DeltaSeconds :type "Float (single-precision)"))
  (if (>= (- (`self.GetGameTimeSinceCreation`) (`self.startTime`)) 5.0)
    (`self.K2_DestroyActor`)))

(fn `UserConstructionScript`)